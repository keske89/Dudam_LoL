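; Game instance Blueprint that runs startup setup when the game initializes.
; On Init it shows the mouse cursor, then creates and stores an HttpRequest object to request the clan member list.
; It scans the Champion asset folder through the Asset Registry and maps each texture into ChampIcon, keyed by its name converted to an integer.
; The resulting icon count is printed for debugging.
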(event `self.ReceiveInit`
  (set `PlayerController.bShowMouseCursor` true (`GameplayStatics.GetPlayerController` 0))
  (bind _returnvalue (`|GenericCreateObject` "/Script/Dudam_LOL.HttpRequest" self))
  (bind _output_get (set `self.HttpRequest_Ref` _returnvalue))
  (`HttpRequest.RequestClanMemberList` _output_get)
  (bind (_outassetdata _returnvalue_2) (`AssetRegistry.GetAssetsByPath` (`AssetRegistryHelpers.GetAssetRegistry`) "/Game/Assets/Champion" false true))
  (for _array_element _outassetdata
    (if _returnvalue_2
      (bind _returnvalue_3 (`AssetRegistryHelpers.GetAsset` _array_element))
      (if (`KismetSystemLibrary.IsValid` _returnvalue_3)
        (bind _astexture_2d (cast `Texture2D` _returnvalue_3))
        (`BlueprintMapLibrary.Map_Add` (`self.ChampIcon`) (`KismetStringLibrary.Conv_StringToInt` (`KismetSystemLibrary.GetDisplayName` _returnvalue_3)) _astexture_2d))))
  (`KismetSystemLibrary.PrintString` (`KismetStringLibrary.Conv_IntToString` (`BlueprintMapLibrary.Map_Length` (`self.ChampIcon`)))))